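; Health potion pickup that restores health to the first-person player character on hit.
; It adds one point of health unless the character is already above a fixed threshold, but is consumed either way.
; After printing a debug message and destroying itself, it plays the health bar blink animation through the character's HUD widget reference.
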(event `self.ReceiveHit`
  (params (MyComp :type "PrimitiveComponent Object Reference") (Other :type "Actor Object Reference") (OtherComp :type "PrimitiveComponent Object Reference") (bSelfMoved :type Boolean) (HitLocation :type "Vector Structure") (HitNormal :type "Vector Structure") (NormalImpulse :type "Vector Structure") (Hit :type "HitResult Structure (by ref)"))
  (bind _asbp_first_person_character (cast `/Game/ContentGame/FirstPerson/Blueprints/BP_FirstPersonCharacter` Other))
  (bind _health (`/Game/ContentGame/FirstPerson/Blueprints/BP_FirstPersonCharacter.health` _asbp_first_person_character))
  (if (not (> _health 2.0))
    (set `/Game/ContentGame/FirstPerson/Blueprints/BP_FirstPersonCharacter.health` (+ _health 1.0) _asbp_first_person_character))
  (`KismetSystemLibrary.PrintString` "Health Potion was collected")
  (`self.K2_DestroyActor`)
  ; Blink animation of Health bar
  (bind _aswbp_game (cast `/Game/ContentGame/UI/WBP_Game` (`/Game/ContentGame/FirstPerson/Blueprints/BP_FirstPersonCharacter.HubWidgetRef` _asbp_first_person_character)))
  (`/Game/ContentGame/UI/WBP_Game.PlayHealthBarAnimation` _aswbp_game))

(fn `UserConstructionScript`)