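; BP_NPC is a werewolf enemy that chases, searches for and damages the player.
; A self-restarting Timer event, driven by delays after each move order, prints and checks mesh-to-mesh distance to the player.
; It chases inside SightRadius or beyond HelpZone, keeping it near the player, and otherwise moves to random navigable points, setting State for each mode.
; Hitting the player applies damage and re-enters Timer after a delay.
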(event `self.ReceiveBeginPlay`
  ;[0 0.01022 0.15 0.5] Pipeline
  (`self.Timer`))

(event `Chase`
  ;[0.03277 0.15 0.01368 0.5] Chase
  (set `self.State` 1)
  (`|AIMoveTo` self (0.0 0.0 0.0) (`GameplayStatics.GetPlayerCharacter` 0)
    (:`then`
      (`KismetSystemLibrary.Delay` 2.3)
      (`self.Timer`))))

(event `Searching`
  ;[0 0.15 0.009963 0.5] Searching
  (set `self.State` 0)
  (bind _newparam1 (`self.RandomPosition` (`SceneComponent.K2_GetComponentLocation` (`self.Mesh`))))
  (`|AIMoveTo` self _newparam1 null 1500.0
    (:`then`
      (`KismetSystemLibrary.Delay` 1.7)
      (`self.Timer`))))

(event `Timer`
  (bind _returnvalue (`KismetMathLibrary.Vector_Distance` (`SceneComponent.K2_GetComponentLocation` (`self.Mesh`)) (`SceneComponent.K2_GetComponentLocation` (`Character.Mesh` (`GameplayStatics.GetPlayerCharacter` 0)))))
  ;[0 0.15 0.007918 0.5] TimerEvent
  (`KismetSystemLibrary.PrintString` (`KismetStringLibrary.Conv_DoubleToString` _returnvalue) true true (struct :`G` 0.66 :`B` 1.0 :`A` 1.0) _returnvalue)
  (if (<= _returnvalue (`self.SightRadius`))
    (`self.Chase` :!label _label)
    (elif (> _returnvalue (`self.HelpZone`))
      (goto _label)
      (else
        (`self.Searching`)))))

(event `self.ReceiveHit`
  (params (MyComp :type "PrimitiveComponent Object Reference") (Other :type "Actor Object Reference") (OtherComp :type "PrimitiveComponent Object Reference") (bSelfMoved :type Boolean) (HitLocation :type "Vector Structure") (HitNormal :type "Vector Structure") (NormalImpulse :type "Vector Structure") (Hit :type "HitResult Structure (by ref)"))
  (bind _returnvalue (`GameplayStatics.GetPlayerCharacter` 0))
  ;[0.02577 0.15 0 0.5] Attack of werewolf
  (if (== Other _returnvalue)
    (`GameplayStatics.ApplyDamage` _returnvalue 1.0 null self)
    (`KismetSystemLibrary.Delay` 0.9)
    (`self.Timer`)))

(fn `RandomPosition`
  (params (NewParam :type "Vector Structure"))
  (returns (NewParam1 :type "Vector Structure"))
  (bind _randomlocation (`NavigationSystemV1.K2_GetRandomLocationInNavigableRadius` NewParam 8000.0 null null))
  (return _randomlocation))

(fn `UserConstructionScript`)