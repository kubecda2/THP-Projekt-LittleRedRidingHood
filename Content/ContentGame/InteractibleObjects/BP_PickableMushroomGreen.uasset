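; BP_PickableMushroomGreen is a green mushroom pickup that slows the first-person player on contact.
; On BeginPlay it rolls a random number against PercentageSpawning and destroys itself when the roll fails, so only some placed mushrooms remain.
; When hit by BP_FirstPersonCharacter, it calls ApplySlow on the character, prints a debug message and destroys itself.
; Disconnected leftover nodes, including an ApplyDamage call, never run.
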(event `self.ReceiveBeginPlay`
  ; Spawning
  (if (not (<= (`KismetMathLibrary.RandomIntegerInRange` 0 100) (`self.PercentageSpawning`)))
    (`self.K2_DestroyActor`)))

(event `self.ReceiveHit`
  (params (MyComp :type "PrimitiveComponent Object Reference") (Other :type "Actor Object Reference") (OtherComp :type "PrimitiveComponent Object Reference") (bSelfMoved :type Boolean) (HitLocation :type "Vector Structure") (HitNormal :type "Vector Structure") (NormalImpulse :type "Vector Structure") (Hit :type "HitResult Structure (by ref)"))
  (bind _asbp_first_person_character (cast `/Game/ContentGame/FirstPerson/Blueprints/BP_FirstPersonCharacter` Other))
  (`/Game/ContentGame/FirstPerson/Blueprints/BP_FirstPersonCharacter.ApplySlow` _asbp_first_person_character)
  (`KismetSystemLibrary.PrintString` "GreenMushroom was collected")
  (`self.K2_DestroyActor`))

(fn `UserConstructionScript`)